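; Player character Blueprint handling look, movement, running and puzzle interaction, with a camera fade-in at start.
; IsPausedOrMenu gates axis input and Tick's walk/run speed switch, and is set while Pause is held or on entering a puzzle.
; Inside a puzzle, E signals Puzzle to move the player to or from its point.
; Overlaps store AudioTrigger, but the name-matched, once-per-trigger track playback chain is disconnected and never runs.
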(event Collision|EventActorBeginOverlap
  (params (OtherActor :type Actor%20Object%20Reference))
  ;[1 1 1] AudioPLayer
  (Variables|Default|SetAudioTrigger OtherActor))

(event EventTick
  (params (DeltaSeconds :type Float%20%28single-precision%29))
  (bind _charactermovement (Variables|Character|GetCharacterMovement))
  ;[1 1 1] Non-Direct Gamplay Systems - Run, Jump, Zoom, Pause
  (if (not (Variables|Default|GetIsPausedOrMenu))
    (if (Variables|Default|GetIsRunning)
      (Variables|/Script/Engine.CharacterMovementComponent|SetMaxWalkSpeed _charactermovement 8e+02)
      (else
        (Variables|/Script/Engine.CharacterMovementComponent|SetMaxWalkSpeed _charactermovement 5e+02)))))

(event EventBeginPlay
  (CameraFades|StartCameraFade :self (Game|GetPlayerCameraManager 0) :FromAlpha 1.0 :Duration 5.0))

(event Input|ActionEvents|InputActionSelect
  (params (Key :type Key%20Structure :default "AnyKey"))
  ;[1 1 1] Input Action Boolean Collection
)

(event Input|ActionEvents|InputActionPause
  (params (Key :type Key%20Structure :default "AnyKey"))
  ;[1 1 1] Input Action Boolean Collection
  (:Pressed
    (Variables|Default|SetIsPausedOrMenu true))
  (:Released
    (Variables|Default|SetIsPausedOrMenu false)))

(event Input|ActionEvents|InputActionRun
  (params (Key :type Key%20Structure :default "AnyKey"))
  ;[1 1 1] Input Action Boolean Collection
  (:Pressed
    (Variables|Default|SetIsRunning true))
  (:Released
    (Variables|Default|SetIsRunning false)))

(event Input|AxisEvents|InputAxisMoveLeft/Right
  (params (AxisValue :type Float%20%28single-precision%29))
  ;[1 1 1] Movement Controllers
  (if (not (Variables|Default|GetIsPausedOrMenu))
    (Pawn|Input|AddMovementInput (Math|Vector|GetRightVector (Math|Rotator|MakeRotator 0.0 0.0 (.Yaw (Math|Rotator|BreakRotator (Pawn|GetControlRotation :!class /Script/Engine.Pawn))))) AxisValue false)))

(event Input|AxisEvents|InputAxisMoveForward/Back
  (params (AxisValue :type Float%20%28single-precision%29))
  ;[1 1 1] Movement Controllers
  (if (not (Variables|Default|GetIsPausedOrMenu))
    (Pawn|Input|AddMovementInput (Math|Vector|GetForwardVector (Math|Rotator|MakeRotator 0.0 0.0 (.Yaw (Math|Rotator|BreakRotator (Pawn|GetControlRotation :!class /Script/Engine.Pawn))))) AxisValue false)))

(event Input|AxisEvents|InputAxisLookLeft/Right
  (params (AxisValue :type Float%20%28single-precision%29))
  ;[1 1 1] Movement Controllers
  (if (not (Variables|Default|GetIsPausedOrMenu))
    (Pawn|Input|AddControllerYawInput AxisValue)))

(event Input|AxisEvents|InputAxisLookUp/Down
  (params (AxisValue :type Float%20%28single-precision%29))
  ;[1 1 1] Movement Controllers
  (if (not (Variables|Default|GetIsPausedOrMenu))
    (Pawn|Input|AddControllerPitchInput AxisValue)))

(event Input|KeyboardEvents|E
  (params (Key :type Key%20Structure :default "AnyKey"))
  (:Pressed
    (if (Variables|Default|GetInPuzzle)
      (if (Variables|Default|GetIsPausedOrMenu)
        (Transformation|SetWorldRotation (Variables|Default|GetSight) (Pawn|GetControlRotation :!class /Script/Engine.Pawn) false false)
        (Variables|/Game/LevelFiles/Dome/Demo/DemoAssets/DemoBlueprints/Puzzle0-TheGate.Puzzle0-TheGate_C|SetMovePlayerFromPoint (Variables|Default|GetPuzzle) true)
        (Variables|/Script/Engine.PlayerController|SetbShowMouseCursor (Game|GetPlayerController 0) false)
        (else
          (Variables|Default|SetIsPausedOrMenu true)
          (Variables|/Script/Engine.CameraComponent|SetbUsePawnControlRotation (Variables|Default|GetCamera) false)
          (Variables|/Game/LevelFiles/Dome/Demo/DemoAssets/DemoBlueprints/Puzzle0-TheGate.Puzzle0-TheGate_C|SetMovePlayerToPoint (Variables|Default|GetPuzzle) true))))))

(fn ConstructionScript)