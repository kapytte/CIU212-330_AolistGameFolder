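; Puzzle0-TheGate is a gate puzzle Blueprint that, as built so far, only detects whether the player is giving movement input.
; The Move Forward/Back and Move Left/Right axis events cache their values.
; Tick sets IsReceivingMovement to true when either cached value is non-zero and false otherwise.
; Nothing in this Blueprint acts on that flag yet, and the construction script is empty.
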(event EventTick
  (params (DeltaSeconds :type Float%20%28single-precision%29))
  (if (Math|Boolean|ORBoolean (!= (Variables|Default|GetInputAxisValuesY) 0.0) (!= (Variables|Default|GetInputAxisValuesX) 0.0) false)
    (Variables|Default|SetIsReceivingMovement true)
    (else
      (Variables|Default|SetIsReceivingMovement false))))

(event Input|AxisEvents|InputAxisMoveLeft/Right
  (params (AxisValue :type Float%20%28single-precision%29))
  (Variables|Default|SetInputAxisValuesY AxisValue))

(event Input|AxisEvents|InputAxisMoveForward/Back
  (params (AxisValue :type Float%20%28single-precision%29))
  (Variables|Default|SetInputAxisValuesX AxisValue))

(fn ConstructionScript)