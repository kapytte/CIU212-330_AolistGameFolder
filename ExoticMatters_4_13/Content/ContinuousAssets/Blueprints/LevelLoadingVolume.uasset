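; LevelLoadingVolume is a trigger that swaps streamed greybox levels when any actor begins overlapping it.
; A switch on the LevelToLoad enum picks the level: Station loads the Station map, while Atoll, Cavern, Dome and Bark all load the Hotel map.
; Each branch starts a non-blocking load, unloads UnLoadLevelName, then stores the new name there, so a repeat overlap unloads the same level it requests.
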(event EventBeginPlay)

(event Collision|EventActorBeginOverlap
  (params (OtherActor :type Actor%20Object%20Reference))
  ;[1 1 1] LevelLoadingOnTrigger
  (switch Utilities|FlowControl|Switch|SwitchonLevelEnum (Utilities|Enum|ByteToEnumLevelEnum (Variables|Default|GetLevelToLoad))
    (:NewEnumerator0
      (bind _output_get (Variables|Default|SetLoadLevelName "ExoticMatters_Greybox_Station"))
      (Game|LoadStreamLevel(byName) _output_get true)
      (Game|UnloadStreamLevel(byName) (Variables|Default|GetUnLoadLevelName))
      (Variables|Default|SetUnLoadLevelName "ExoticMatters_Greybox_Station"))
    (:NewEnumerator1
      (bind _output_get_2 (Variables|Default|SetLoadLevelName "ExoticMatters_Greybox_Hotel"))
      (Game|LoadStreamLevel(byName) _output_get_2 true)
      (Game|UnloadStreamLevel(byName) (Variables|Default|GetUnLoadLevelName))
      (Variables|Default|SetUnLoadLevelName "ExoticMatters_Greybox_Hotel"))
    (:NewEnumerator3
      (bind _output_get_3 (Variables|Default|SetLoadLevelName "ExoticMatters_Greybox_Hotel"))
      (Game|LoadStreamLevel(byName) _output_get_3 true)
      (Game|UnloadStreamLevel(byName) (Variables|Default|GetUnLoadLevelName))
      (Variables|Default|SetUnLoadLevelName "ExoticMatters_Greybox_Hotel"))
    (:NewEnumerator4
      (bind _output_get_4 (Variables|Default|SetLoadLevelName "ExoticMatters_Greybox_Hotel"))
      (Game|LoadStreamLevel(byName) _output_get_4 true)
      (Game|UnloadStreamLevel(byName) (Variables|Default|GetUnLoadLevelName))
      (Variables|Default|SetUnLoadLevelName "ExoticMatters_Greybox_Hotel"))
    (:NewEnumerator6
      (bind _output_get_5 (Variables|Default|SetLoadLevelName "ExoticMatters_Greybox_Hotel"))
      (Game|LoadStreamLevel(byName) _output_get_5 true)
      (Game|UnloadStreamLevel(byName) (Variables|Default|GetUnLoadLevelName))
      (Variables|Default|SetUnLoadLevelName "ExoticMatters_Greybox_Hotel"))))

(event EventTick
  (params (DeltaSeconds :type Float%20%28single-precision%29)))

(fn ConstructionScript)