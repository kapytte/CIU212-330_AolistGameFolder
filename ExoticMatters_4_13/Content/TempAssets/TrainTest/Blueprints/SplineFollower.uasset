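; Train-test spline follower actor, meant to step along the points of a referenced Spline actor.
; BeginPlay places its root at the current point's X, Y and rotation.
; Pressing W caches current and next point transforms, then advances the index, wrapping to zero at the end.
; The transform-lerp move between those points is unconnected and Tick is empty, so the actor stays put after BeginPlay.
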(event EventBeginPlay
  (bind _currentsplinepointnumber (Variables|Default|GetCurrentSplinePointNumber))
  (bind _asspline (Utilities|Casting|CastToSpline (Variables|Default|GetActor%20Referance)))
  (Variables|Default|SetActor%20Referance _asspline)
  (Transformation|SetWorldLocationAndRotation (Variables|Default|GetDefaultSceneRoot) (Math|Vector|MakeVector (.x (Spline|GetLocationatSplinePoint (Variables|/Game/TempAssets/TrainTest/Blueprints/Spline.Spline_C|GetSpline _asspline) _currentsplinepointnumber "World")) (.y (Spline|GetLocationatSplinePoint (Variables|/Game/TempAssets/TrainTest/Blueprints/Spline.Spline_C|GetSpline _asspline) _currentsplinepointnumber "World")) 0.0) (Spline|GetRotationatSplinePoint (Variables|/Game/TempAssets/TrainTest/Blueprints/Spline.Spline_C|GetSpline _asspline) _currentsplinepointnumber "World") true false))

(event EventTick
  (params (DeltaSeconds :type Float%20%28single-precision%29)))

(event Input|KeyboardEvents|W
  (params (Key :type Key%20Structure :default "AnyKey"))
  (:Pressed
    (bind _asspline (Utilities|Casting|CastToSpline (Variables|Default|GetActor%20Referance)))
    (bind _output_get (Variables|Default|SetCurrentSplinePoint (Math|Transform|MakeTransform (Spline|GetLocationatSplinePoint (Variables|/Game/TempAssets/TrainTest/Blueprints/Spline.Spline_C|GetSpline _asspline) (Variables|Default|GetCurrentSplinePointNumber) "World") (Spline|GetRotationatSplinePoint (Variables|/Game/TempAssets/TrainTest/Blueprints/Spline.Spline_C|GetSpline _asspline) (Variables|Default|GetCurrentSplinePointNumber) "World") "1,1,1")))
    (bind _output_get_2 (Variables|Default|SetNextSplinePoint (Math|Transform|MakeTransform (Spline|GetLocationatSplinePoint (Variables|/Game/TempAssets/TrainTest/Blueprints/Spline.Spline_C|GetSpline _asspline) (+ (Variables|Default|GetCurrentSplinePointNumber) 1) "World") (Spline|GetRotationatSplinePoint (Variables|/Game/TempAssets/TrainTest/Blueprints/Spline.Spline_C|GetSpline _asspline) (+ (Variables|Default|GetCurrentSplinePointNumber) 1) "World") "1,1,1")))
    (if (>= (+ (Variables|Default|GetCurrentSplinePointNumber) 1) (Spline|GetNumberOfSplinePoints (Variables|/Game/TempAssets/TrainTest/Blueprints/Spline.Spline_C|GetSpline _asspline)))
      (Variables|Default|SetCurrentSplinePointNumber 0)
      (else
        (Variables|Default|SetCurrentSplinePointNumber (+ (Variables|Default|GetCurrentSplinePointNumber) 1))))))

(fn ConstructionScript)