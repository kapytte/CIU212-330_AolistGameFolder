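; Test train actor that rides along one of two referenced track splines, with W switching to the second track and S back to the first.
; BeginPlay takes the starting distance from a destination spline point on track one.
; Each Tick picks the active spline, adds Speed without delta-time scaling, wraps to zero at the end, then sweeps the root to that distance.
; Location uses only the spline's X and Y, while rotation follows the spline.
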(event EventBeginPlay
  ;[1 1 1] Set the intital Spline Position
  (bind _output_get (Variables|Default|SetCurrentSplinePath (Variables|/Game/TempAssets/TrainTest/Blueprints/Track1Spline.Track1Spline_C|GetSpline (Variables|Default|GetTrack1SplineReference))))
  (Variables|Default|SetSplineDistance (Spline|GetDistanceAlongSplineatSplinePoint _output_get (Variables|Default|GetDesitnationSplinePoint)))
  (CallFunction|UpdateSpline))

(event Collision|EventActorBeginOverlap
  (params (OtherActor :type Actor%20Object%20Reference)))

(event EventTick
  (params (DeltaSeconds :type Float%20%28single-precision%29))
  (if (Variables|Default|GetGoToNextSpline)
    (Variables|Default|SetCurrentSplinePath (Variables|/Game/TempAssets/TrainTest/Blueprints/Track2Spline.Track2Spline_C|GetSpline (Variables|Default|GetTrack2SplineReference)))
    (else
      (Variables|Default|SetCurrentSplinePath (Variables|/Game/TempAssets/TrainTest/Blueprints/Track1Spline.Track1Spline_C|GetSpline (Variables|Default|GetTrack1SplineReference)))))
  (CallFunction|MovementControl)
  (CallFunction|UpdateSpline))

(event Input|KeyboardEvents|W
  (params (Key :type Key%20Structure :default "AnyKey"))
  (:Pressed
    (Variables|Default|SetGoToNextSpline true)))

(event Input|KeyboardEvents|S
  (params (Key :type Key%20Structure :default "AnyKey"))
  (:Pressed
    (Variables|Default|SetGoToNextSpline false)))

(fn ConstructionScript)

(fn UpdateSpline
  (bind _currentsplinepath (Variables|Default|GetCurrentSplinePath))
  (bind _splinedistance (Variables|Default|GetSplineDistance))
  (bind _returnvalue (Spline|GetLocationatDistanceAlongSpline _currentsplinepath _splinedistance "World"))
  (Transformation|SetWorldLocationAndRotation (Variables|Default|GetDefaultSceneRoot) (Math|Vector|MakeVector (.x _returnvalue) (.y _returnvalue) 0.0) (Spline|GetRotationatDistanceAlongSpline _currentsplinepath _splinedistance "World") true false))

(fn MovementControl
  (Variables|Default|SetSplineDistance (+ (Variables|Default|GetSplineDistance) (Variables|Default|GetSpeed)))
  (if (>= (Variables|Default|GetSplineDistance) (Spline|GetSplineLength (Variables|Default|GetCurrentSplinePath)))
    (Variables|Default|SetSplineDistance 0.0)))