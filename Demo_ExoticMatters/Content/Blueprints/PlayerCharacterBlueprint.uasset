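; Player character Blueprint that handles look, movement, running, jumping and zoom from player input.
; Axis events drive look and movement directly, while action events only set boolean flags.
; Tick reads those flags to switch walk speed, trigger a one-shot jump and narrow the camera FOV for zoom.
; A pause flag, true only while Pause is held, gates both axis input and the Tick logic without pausing the game itself.
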(event EventTick
  (params (DeltaSeconds :type Float%20%28single-precision%29))
  (bind _camera (Variables|Default|GetCamera))
  (bind _charactermovement (Variables|Character|GetCharacterMovement))
  ;[1 1 1] Non-Direct Gamplay Systems - Run, Jump, Zoom, Pause
  (if (not (Variables|Default|GetIsPausedOrMenu))
    (if (Variables|Default|GetIsRunning)
      (Variables|/Script/Engine.CharacterMovementComponent|SetMaxWalkSpeed _charactermovement 8e+02)
      (else
        (Variables|/Script/Engine.CharacterMovementComponent|SetMaxWalkSpeed _charactermovement 5e+02)))
    (if (Variables|Default|GetIsJumping)
      (Character|Jump)
      (Variables|Default|SetIsJumping false))
    (if (Variables|Default|GetIsZoomed)
      (Camera|SetFieldOfView _camera 8e+01)
      (else
        (Camera|SetFieldOfView _camera 9e+01)))))

(event Input|ActionEvents|InputActionSelect
  (params (Key :type Key%20Structure :default "AnyKey"))
  ;[1 1 1] Input Action Boolean Collection
)

(event Input|ActionEvents|InputActionJump
  (params (Key :type Key%20Structure :default "AnyKey"))
  ;[1 1 1] Input Action Boolean Collection
  (:Pressed
    (Variables|Default|SetIsJumping true)))

(event Input|ActionEvents|InputActionPause
  (params (Key :type Key%20Structure :default "AnyKey"))
  ;[1 1 1] Input Action Boolean Collection
  (:Pressed
    (Variables|Default|SetIsPausedOrMenu true))
  (:Released
    (Variables|Default|SetIsPausedOrMenu false)))

(event Input|ActionEvents|InputActionZoomLook
  (params (Key :type Key%20Structure :default "AnyKey"))
  ;[1 1 1] Input Action Boolean Collection
  (:Pressed
    (Variables|Default|SetIsZoomed true))
  (:Released
    (Variables|Default|SetIsZoomed false)))

(event Input|ActionEvents|InputActionRun
  (params (Key :type Key%20Structure :default "AnyKey"))
  ;[1 1 1] Input Action Boolean Collection
  (:Pressed
    (Variables|Default|SetIsRunning true))
  (:Released
    (Variables|Default|SetIsRunning false)))

(event Input|AxisEvents|InputAxisMoveLeft/Right
  (params (AxisValue :type Float%20%28single-precision%29))
  ;[1 1 1] Movement Controllers
  (if (not (Variables|Default|GetIsPausedOrMenu))
    (Pawn|Input|AddMovementInput (Transformation|GetActorRightVector) AxisValue false)))

(event Input|AxisEvents|InputAxisMoveForward/Back
  (params (AxisValue :type Float%20%28single-precision%29))
  ;[1 1 1] Movement Controllers
  (if (not (Variables|Default|GetIsPausedOrMenu))
    (Pawn|Input|AddMovementInput (Transformation|GetActorForwardVector) AxisValue false)))

(event Input|AxisEvents|InputAxisLookLeft/Right
  (params (AxisValue :type Float%20%28single-precision%29))
  ;[1 1 1] Movement Controllers
  (if (not (Variables|Default|GetIsPausedOrMenu))
    (Pawn|Input|AddControllerYawInput AxisValue)))

(event Input|AxisEvents|InputAxisLookUp/Down
  (params (AxisValue :type Float%20%28single-precision%29))
  ;[1 1 1] Movement Controllers
  (if (not (Variables|Default|GetIsPausedOrMenu))
    (Pawn|Input|AddControllerPitchInput AxisValue)))

(fn ConstructionScript)